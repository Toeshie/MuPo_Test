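; BP_SpawnerTest is a test spawner that spawns high or low note actors from timed events in the SongData table.
; BeginPlay splits rows into time, action and note-number arrays and starts a looping NoteProcess timer.
; NoteProcess accumulates frame delta per timer tick, then nests loops over the arrays instead of sharing one index, removing entries mid-loop.
; Due spawn events at or above the note threshold spawn LowNoteRef, others HighNoteRef.
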(event EventBeginPlay
  (Variables|Default|SetUsedTimeDelta 0.0)
  (bind _outrownames (DataTable|GetDataTableRowNames (Variables|Default|GetSongData)))
  (for _array_element _outrownames
    (bind _returnvalue (Utilities|GetDataTableRow (Variables|Default|GetSongData) _array_element)
      (:then
        (bind _output_get (Variables|Default|SetDelayInSeconds (/ (.Time_ms (Utilities|Struct|BreakNoteInfo_Stuct _returnvalue)) (Variables|Default|GetSecondConverterValue))))
        (Utilities|Array|Add (Variables|Default|GetTimeArray) _output_get)
        (Utilities|Array|Add (Variables|Default|GetSpawnEventsArray) (.Action (Utilities|Struct|BreakNoteInfo_Stuct _returnvalue)))
        (Utilities|Array|Add (Variables|Default|GetNoteNumberArray) (.Note_Number (Utilities|Struct|BreakNoteInfo_Stuct _returnvalue)))
        (Utilities|Time|SetTimerbyFunctionName 0 "NoteProcess" 0.05 true)))))

(fn ConstructionScript)

(fn SpawnNote
  (Game|SpawnActorfromClass (Variables|Default|GetLowNoteRef) (Variables|Default|GetSpawn%20Transform) "Undefined" "MultiplyWithRoot" 0 0))

(fn SpawnNoteHigh
  (Game|SpawnActorfromClass (Variables|Default|GetHighNoteRef) (Variables|Default|GetSpawn%20Transform_0) "Undefined" "MultiplyWithRoot" 0 0))

(fn NoteProcess
  (bind _output_get (Variables|Default|SetUsedTimeDelta (+ (Utilities|Time|GetWorldDeltaSeconds) (Variables|Default|GetUsedTimeDelta))))
  (for (_array_element _array_index) (Variables|Default|GetNoteNumberArray)
    (for (_array_element_2 _array_index_2) (Variables|Default|GetSpawnEventsArray)
      (for (_array_element_3 _array_index_3) (Variables|Default|GetTimeArray)
        (if (Utilities|Enum|Equal(Enum) _array_element_2 (Variables|Default|GetSpawnEvent))
          (if (>= _output_get _array_element_3)
            (if (>= _array_element (Variables|Default|GetNoteNumberTreshold))
              (CallFunction|SpawnNote)
              (else
                (CallFunction|SpawnNoteHigh)))
            (Utilities|Array|RemoveIndex (Variables|Default|GetTimeArray) _array_index_3)
            (Utilities|Array|RemoveIndex (Variables|Default|GetSpawnEventsArray) _array_index_2)
            (Utilities|Array|RemoveIndex (Variables|Default|GetNoteNumberArray) _array_index))
          (else
            (Utilities|Array|RemoveIndex (Variables|Default|GetSpawnEventsArray) _array_index_2)))))))