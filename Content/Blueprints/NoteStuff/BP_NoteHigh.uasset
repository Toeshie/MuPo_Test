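; BP_NoteHigh is a note actor, apparently the high variant, that is positioned on a spline and destroys itself.
; BeginPlay sets the start distance from a reset value and caches the spline length.
; Tick places it at start distance plus the frame's speed step, without using the running total.
; That same sum accumulates separately, and the actor is destroyed once the total reaches the spline length.
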(event EventBeginPlay
  (Variables|Default|SetDistanceAlongSpline (Variables|Default|GetReset%20Value))
  (bind _output_get (Variables|Default|SetSplineLenght (Spline|GetSplineLength (Variables|Default|GetSpline)))))

(event EventTick
  (params (DeltaSeconds :type Float%20%28single-precision%29))
  (bind _speed (Variables|Default|GetSpeed))
  (bind _distancealongspline (Variables|Default|GetDistanceAlongSpline))
  (bind _returnvalue (* DeltaSeconds _speed))
  (bind _returnvalue_2 (+ _distancealongspline _returnvalue))
  (bind _output_get (Variables|Default|SetCurrentDistance (+ _returnvalue_2 (Variables|Default|GetCurrentDistance))))
  (Transformation|SetActorLocation (Spline|GetLocationatDistanceAlongSpline (Variables|Default|GetSpline) _returnvalue_2 "World") false false)
  (if (>= _output_get (stale EventBeginPlay _output_get))
    (Actor|DestroyActor)))

(fn ConstructionScript)