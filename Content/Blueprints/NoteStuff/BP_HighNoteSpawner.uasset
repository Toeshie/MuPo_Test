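; BP_HighNoteSpawner spawns note actors at times read from a song data table, using the LowNoteRef class despite its high-note name.
; On BeginPlay it scans SongData rows, converts TimeMs of those matching SpawnEvent to seconds, and prints each delay.
; Each match sets a SpawnNote timer by function name, so each call resets the previous one rather than queuing another spawn.
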(event EventBeginPlay
  (bind _outrownames (DataTable|GetDataTableRowNames (Variables|Default|GetSongData)))
  (for _array_element _outrownames
    (bind _returnvalue (Utilities|GetDataTableRow (Variables|Default|GetSongData) _array_element)
      (:then
        (if (Utilities|Enum|Equal(Enum) (.Action (Utilities|Struct|BreakNoteInfo_Stuct _returnvalue)) (Variables|Default|GetSpawnEvent))
          (bind _output_get (Variables|Default|SetDelayInSeconds (/ (.Time_ms (Utilities|Struct|BreakNoteInfo_Stuct _returnvalue)) (Variables|Default|GetSecondConverterValue))))
          (Utilities|Time|SetTimerbyFunctionName 0 "SpawnNote" _output_get)
          (Development|PrintString (Utilities|String|ToString(Float) _output_get) true true "(R=0.000000,G=0.660000,B=1.000000,A=1.000000)" _output_get))))))

(fn ConstructionScript)

(fn SpawnNote
  (Game|SpawnActorfromClass (Variables|Default|GetLowNoteRef) (Variables|Default|GetSpawn%20Transform) "Undefined" "MultiplyWithRoot" 0 0))